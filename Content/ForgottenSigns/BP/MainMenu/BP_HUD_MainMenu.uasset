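; Main menu HUD that shows the start menu when the level begins.
; On BeginPlay it creates the UI_StartMainMenu widget, stores it and adds it to the player screen.
; It then shows the mouse cursor and switches the owning player controller to UI-only input without mouse lock.
; A HideMouseCursor function reverses this to game-only input but is not called within this Blueprint.
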(event EventBeginPlay
  (Init|InitStartMainMenu)
  (MouseCursor|ShowMouseCursor))

(fn ConstructionScript)

(fn InitStartMainMenu
  (bind _returnvalue (UserInterface|CreateWidget "/Game/ForgottenSigns/BP/MainMenu/UI_StartMainMenu.UI_StartMainMenu_C"))
  (bind _output_get (Variables|Default|SetStartMainMenu _returnvalue))
  (UserInterface|Viewport|AddtoPlayerScreen _output_get))

(fn ShowMouseCursor
  (bind _returnvalue (Game|Player|GetOwningPlayerController))
  (Variables|/Script/Engine.PlayerController|SetbShowMouseCursor _returnvalue true)
  (Input|SetInputModeUIOnly _returnvalue 0 "DoNotLock"))

(fn HideMouseCursor
  (bind _returnvalue (Game|Player|GetOwningPlayerController))
  (Variables|/Script/Engine.PlayerController|SetbShowMouseCursor _returnvalue false)
  (Input|SetInputModeGameOnly _returnvalue))