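; Default player HUD that creates the player UI widget and shows an interaction prompt.
; On BeginPlay it adds a UI_PlayerDefault widget to the owning player's screen and caches the owning pawn as a DefaultPlayer.
; Every Tick it polls the player's CanInteractive flag to show and enable, or hide and disable, the widget's use text.
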(event EventBeginPlay
  (CallFunction|AddUIPlayerDefault)
  (CallFunction|InitDefaultPlayer))

(event EventTick
  (params (DeltaSeconds :type Float%20%28single-precision%29))
  (CallFunction|ShowUseText))

(fn ConstructionScript)

(fn ShowUseText
  (bind _currentuiplayerdefault (Variables|Default|GetcurrentUIPlayerDefault))
  (bind _currentuiplayerdefault_2 (Variables|Default|GetcurrentUIPlayerDefault))
  (bind _textuse (Variables|/Game/ForgottenSigns/BP/Player/UI_PlayerDefault.UI_PlayerDefault_C|GettextUse _currentuiplayerdefault))
  (bind _textuse_2 (Variables|/Game/ForgottenSigns/BP/Player/UI_PlayerDefault.UI_PlayerDefault_C|GettextUse _currentuiplayerdefault_2))
  (if (Variables|/Script/ForgottenSigns.DefaultPlayer|GetcanInteractive (Variables|Default|Getplayer))
    (Widget|SetIsEnabled _textuse_2 true)
    (Widget|SetVisibility _textuse_2 "Visible")
    (else
      (Widget|SetVisibility _textuse "Hidden")
      (Widget|SetIsEnabled _textuse false))))

(fn AddUIPlayerDefault
  (bind _returnvalue (UserInterface|CreateWidget "/Game/ForgottenSigns/BP/Player/UI_PlayerDefault.UI_PlayerDefault_C" (Variables|Default|GetPlayerOwner)))
  (bind _output_get (Variables|Default|SetcurrentUIPlayerDefault _returnvalue))
  (UserInterface|Viewport|AddtoPlayerScreen _output_get))

(fn InitDefaultPlayer
  (bind _asdefault_player (Utilities|Casting|CastToDefaultPlayer (Class|HUD|GetOwningPawn)))
  (Variables|Default|Setplayer _asdefault_player))