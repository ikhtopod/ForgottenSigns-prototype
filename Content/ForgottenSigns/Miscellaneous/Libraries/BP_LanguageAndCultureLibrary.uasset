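; Blueprint function library for setting the game's culture, limited to cultures the project is localized for.
; InitDefaultCulture takes the first two characters of the default language as a culture code and passes it to UpdateCulture.
; UpdateCulture sets the current culture if that code is among the localized cultures, optionally saving it to config, and otherwise returns false.
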(fn InitDefaultCulture
  (params (SaveToConfig :type Boolean))
  (bind _returnvalue (Utilities|Internationalization|BP_LanguageAndCultureLibrary|UpdateCulture (Utilities|String|GetSubstring (Class|KismetSystemLibrary|GetDefaultLanguage) 0 2) SaveToConfig))
  (return _returnvalue))

(fn UpdateCulture
  (params (cultureName :type String) (SaveToConfig :type Boolean))
  (bind _returnvalue (Class|KismetInternationalizationLibrary|GetLocalizedCultures true false false false))
  (bind _returnvalue_2 (Utilities|Array|FindItem _returnvalue cultureName))
  (if (>= _returnvalue_2 0)
    (bind _returnvalue_3 (Class|KismetInternationalizationLibrary|SetCurrentCulture (Utilities|Array|Get(acopy) _returnvalue _returnvalue_2) SaveToConfig))
    (return _returnvalue_3)
    (else
      (return false))))