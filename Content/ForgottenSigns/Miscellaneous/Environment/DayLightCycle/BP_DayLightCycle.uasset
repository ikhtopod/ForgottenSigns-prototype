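; BP_DayLightCycle is the day/night cycle actor, combining a sky sphere, a directional light and exponential height fog.
; On BeginPlay it caches the sky sphere and light child actors, links the light to the sky material and passes its Speed to the light's rotation.
; Each tick it sets fog max opacity from the sky sphere's sun height, with separate day and night offsets, clamped between zero and one.
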(event EventBeginPlay
  (Utilities|FlowControl|Sequence
    (:then_0
      (CallFunction|InitSkySphere)
      (CallFunction|InitDirectionalLight))
    (:then_1
      (CallFunction|AssignDirectionalLighttoSkySphere)
      (CallFunction|AssignSpeedRotation))))

(event EventTick
  (params (DeltaSeconds :type Float%20%28single-precision%29))
  (CallFunction|UpdateExponentialHeightFog))

(fn ConstructionScript)

(fn UpdateExponentialHeightFog
  (bind _output_get (LocalVariables|SetsunHeight (Variables|/Game/ForgottenSigns/Miscellaneous/Environment/DayLightCycle/BP_DayLightCycle_SkySphere.BP_DayLightCycle_SkySphere_C|GetSun%20height (Variables|Default|GetskySphere))))
  (if (< _output_get 0.0)
    (LocalVariables|SetdayNightMult 0.4) ; night
    (else
      (LocalVariables|SetdayNightMult 0.6) ; day
    ))
  (LocalVariables|SetnewOpacity (Math|Float|Clamp(Float) (+ (* (LocalVariables|GetsunHeight) 0.6) (LocalVariables|GetdayNightMult)) 0.0))
  (Class|ExponentialHeightFogComponent|SetFogMaxOpacity (Variables|Default|GetExponentialHeightFog) (LocalVariables|GetnewOpacity)))

(fn InitSkySphere
  (bind _asbp_day_light_cycle_sky_sphere (Utilities|Casting|CastToBP_DayLightCycle_SkySphere (Variables|/Script/Engine.ChildActorComponent|GetChildActor (Variables|Default|GetBP_DayLightCycle_SkySphere))))
  (Variables|Default|SetskySphere _asbp_day_light_cycle_sky_sphere))

(fn InitDirectionalLight
  (bind _asbp_day_light_cycle_directional_light (Utilities|Casting|CastToBP_DayLightCycle_DirectionalLight (Variables|/Script/Engine.ChildActorComponent|GetChildActor (Variables|Default|GetBP_DayLightCycle_DirectionalLight))))
  (Variables|Default|SetdirectionalLight _asbp_day_light_cycle_directional_light))

(fn AssignDirectionalLighttoSkySphere
  (bind _skysphere (Variables|Default|GetskySphere))
  (Variables|/Game/ForgottenSigns/Miscellaneous/Environment/DayLightCycle/BP_DayLightCycle_SkySphere.BP_DayLightCycle_SkySphere_C|SetDirectional%20light%20actor _skysphere (Variables|Default|GetdirectionalLight))
  (Default|RefreshMaterial _skysphere))

(fn AssignSpeedRotation
  (Default|SetSpeedRotation (Variables|Default|GetdirectionalLight) (Variables|Default|Getspeed)))