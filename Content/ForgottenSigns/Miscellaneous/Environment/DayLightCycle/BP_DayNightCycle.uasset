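; BP_DayNightCycle drives the level's day-night cycle through a timeline that animates sun, sky and fog.
; Tick applies timeline values to directional light rotation and intensity, sky light intensity and height fog density, then updates the sky sphere's sun direction.
; It also builds a Timespan from the day and timeline position.
; A looping timer periodically recaptures the sky light; DayTickSystem is an empty stub.
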(event Custom|RecaptureSkyLight
  ;[1 1 1] Recapture Sky
  (Class|SkyLightComponent|RecaptureSky (Variables|/Script/Engine.SkyLight|GetLightComponent (Variables|Default|GetskyLight))))

(event EventBeginPlay
  (Utilities|FlowControl|Sequence
    (:then_0
      (bind (_direction _directionallightrotationpitch _directionallightrotationyaw _time _skylightintensity _exponentialheightfogdensity _directionallightintensity) (Timeline|DayLightCycle_Timeline SetNewTime)))
    (:then_1
      ;[1 1 1] Recapture Sky
      (Utilities|Time|SetTimerbyEvent (delegate Custom|RecaptureSkyLight) 5.0 true))))

(event EventTick
  (params (DeltaSeconds :type Float%20%28single-precision%29))
  (CallFunction|UpdateTime)
  (Variables|Default|SetsecondTimeTimeline (stale EventBeginPlay _time))
  (Transformation|SetActorRotation (Variables|Default|GetdirectionalLight) (Math|Rotator|MakeRotator 0.0 (stale EventBeginPlay _directionallightrotationpitch) (stale EventBeginPlay _directionallightrotationyaw)))
  (Rendering|Components|Light|SetIntensity (Variables|/Script/Engine.SkyLight|GetLightComponent (Variables|Default|GetskyLight)) (stale EventBeginPlay _skylightintensity))
  (Class|ExponentialHeightFogComponent|SetFogDensity (Variables|/Script/Engine.ExponentialHeightFog|GetComponent (Variables|Default|GetexponentialHeightFog)) (stale EventBeginPlay _exponentialheightfogdensity))
  (Rendering|Components|Light|SetIntensity (Variables|/Script/Engine.Light|GetLightComponent (Variables|Default|GetdirectionalLight)) (stale EventBeginPlay _directionallightintensity))
  (Default|UpdateSunDirection (Variables|Default|GetskySphere)))

(fn ConstructionScript)

(fn UpdateTime
  (Variables|Default|Settime (Math|Timespan|MakeTimespan (Variables|Default|Getday) 0 0 (Math|Float|Truncate (Variables|Default|GetsecondTimeTimeline)))))

(fn DayTickSystem)