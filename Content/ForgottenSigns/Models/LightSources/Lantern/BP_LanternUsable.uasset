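; BP_LanternUsable is a usable lantern rig that raises the lantern into place and lights it, or lowers and hides it, when toggled.
; A child actor component supplies the BP_Lantern, whose IsLighting state sets the spring arm's starting height and visibility and picks the toggle direction.
; A timeline lerps the spring arm's relative Z, switching the light on after the raise and off, with the arm hidden, after the reverse.
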(event EventToggleLantern
  ;[1 1 1] Toggle Lantern
  (if (not (Variables|/Game/ForgottenSigns/Models/LightSources/Lantern/BP_Lantern.BP_Lantern_C|GetisLighting (Variables|Lantern|GetLanternActor)))
    (Rendering|SetVisibility (Variables|Default|GetLanternSpringArm) true true)
    (bind (_direction _alpha) (Timeline|Timeline_0 Play)
      (:Update
        (LanternTimeline|LanternTimelineUpdate _alpha))
      (:Finished
        (LanternTimeline|LanternTimelineFinish _direction)))
    (else
      (Timeline|Timeline_0 Reverse))))

(event EventBeginPlay
  (Lantern|InitLanternActor)
  (Lantern|InitStartLocationLanternSpringArm)
  (Lantern|BeginLanternSpringArmPosition))

(fn ConstructionScript)

(fn InitLanternActor
  (bind _asbp_lantern (Utilities|Casting|CastToBP_Lantern (Variables|/Script/Engine.ChildActorComponent|GetChildActor (Variables|Default|GetLanternActorComponent))))
  (Variables|Lantern|SetLanternActor _asbp_lantern))

(fn InitStartLocationLanternSpringArm
  (Variables|Lantern|SetstartLocationLanternSpringArm (Variables|/Script/Engine.SceneComponent|GetRelativeLocation (Variables|Default|GetLanternSpringArm))))

(fn BeginLanternSpringArmPosition
  (bind _lanternactor (Variables|Lantern|GetLanternActor))
  (bind _startlocationlanternspringarm (Variables|Lantern|GetstartLocationLanternSpringArm))
  (bind _islighting (Variables|/Game/ForgottenSigns/Models/LightSources/Lantern/BP_Lantern.BP_Lantern_C|GetisLighting _lanternactor))
  (Rendering|SetVisibility (Variables|Default|GetLanternSpringArm) _islighting true)
  (if _islighting
    (Transformation|SetRelativeLocation (Variables|Default|GetLanternSpringArm) (Variables|Lantern|GetstartLocationLanternSpringArm) false false)
    (else
      (Transformation|SetRelativeLocation (Variables|Default|GetLanternSpringArm) (Math|Vector|MakeVector (.x _startlocationlanternspringarm) (.y _startlocationlanternspringarm) (- (.z _startlocationlanternspringarm) (Variables|Lantern|GetlanternOffset))) false false))))

(fn LanternTimelineUpdate
  (params (alpha :type Float%20%28single-precision%29))
  (bind _lanternspringarm (Variables|Default|GetLanternSpringArm))
  (bind _startlocationlanternspringarm (Variables|Lantern|GetstartLocationLanternSpringArm))
  (bind _relativelocation (Variables|/Script/Engine.SceneComponent|GetRelativeLocation _lanternspringarm))
  (Transformation|SetRelativeLocation _lanternspringarm (Math|Vector|MakeVector (.x _relativelocation) (.y _relativelocation) (Math|Float|Lerp (- (.z _startlocationlanternspringarm) (Variables|Lantern|GetlanternOffset)) (.z _startlocationlanternspringarm) alpha)) false false))

(fn LanternTimelineFinish
  (params (direction :type ETimelineDirection%20Enum :default "Forward"))
  (bind _lanternactor (Variables|Lantern|GetLanternActor))
  (if (Utilities|Enum|Equal(Enum) direction "Forward")
    (Default|Lighton _lanternactor)
    (else
      (Default|LightOff _lanternactor)
      (Rendering|SetVisibility (Variables|Default|GetLanternSpringArm) false true))))