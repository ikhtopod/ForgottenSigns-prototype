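; BP_FloorLamp_01 is an interactable floor lamp whose light can be switched on and off.
; Interact flips IsLighting when CanLighting allows it, then UpdateFloorLamp applies that state to the visibility of the PointLight and its children.
; The construction script and BeginPlay run the same update, keeping the light in sync with IsLighting at construction and at game start.
; GetWidgetComponent exposes the interact icon widget component.
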(event EventInteract
  (CallFunction|ToggleFloorLamp))

(event EventBeginPlay
  (CallFunction|UpdateFloorLamp))

(fn ConstructionScript
  (CallFunction|UpdateFloorLamp))

(fn UpdateFloorLamp
  (Rendering|SetVisibility (Variables|Default|GetPointLight) (Variables|Default|GetisLighting) true))

(fn ToggleFloorLamp
  (if (Variables|Default|GetcanLighting)
    (Variables|Default|SetisLighting (not (Variables|Default|GetisLighting)))
    (CallFunction|UpdateFloorLamp)))

(fn GetWidgetComponent
  (return (Variables|Default|GetInteractIconWidgetComponent)))