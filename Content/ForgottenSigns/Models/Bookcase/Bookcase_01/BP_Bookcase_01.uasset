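; Bookcase prop built from three BP_Bookshelf_01 child actors, with a HasBooks setting shared by all shelves.
; The construction script casts each child actor component's actor to BP_Bookshelf_01 and caches it in a variable.
; It then copies the bookcase's HasBooks value onto each cached shelf.
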(fn ConstructionScript
  (Bookshelf|InitBookshelvesActor)
  (Bookshelf|UpdateBookshelfHasBooks))

(fn InitBookshelvesActor
  (Utilities|FlowControl|Sequence
    (:then_0
      (bind _asbp_bookshelf_01 (Bookshelf|CastComponenttoActor (Variables|Default|GetBP_Bookshelf_01)))
      (Variables|Bookshelf|SetbookshelfActor_01 _asbp_bookshelf_01))
    (:then_1
      (bind _asbp_bookshelf_01_2 (Bookshelf|CastComponenttoActor (Variables|Default|GetBP_Bookshelf_02)))
      (Variables|Bookshelf|SetbookshelfActor_02 _asbp_bookshelf_01_2))
    (:then_2
      (bind _asbp_bookshelf_01_3 (Bookshelf|CastComponenttoActor (Variables|Default|GetBP_Bookshelf_03)))
      (Variables|Bookshelf|SetbookshelfActor_03 _asbp_bookshelf_01_3))))

(fn CastComponenttoActor
  (params (childActorComponent :type Child%20Actor%20Component%20Object%20Reference%20%28by%20ref%29))
  (bind _asbp_bookshelf_01 (Utilities|Casting|CastToBP_Bookshelf_01 (Variables|/Script/Engine.ChildActorComponent|GetChildActor childActorComponent)))
  (return _asbp_bookshelf_01))

(fn UpdateBookshelfHasBooks
  (for _array_element (Utilities|Array|MakeArray (Variables|Bookshelf|GetbookshelfActor_01) (Variables|Bookshelf|GetbookshelfActor_02) (Variables|Bookshelf|GetbookshelfActor_03))
    (Variables|/Game/ForgottenSigns/Models/Bookcase/Bookcase_01/BP_Bookshelf_01.BP_Bookshelf_01_C|SethasBooks _array_element (Variables|Bookshelf|GethasBooks))))