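; Interactable door Blueprint that swings open and closed when the player interacts with it.
; Interact fires a toggle that plays or reverses a rotation timeline, driving the door mesh's relative yaw while keeping roll and pitch.
; A CanOpen flag blocks re-triggering mid-swing, and the timeline's finish flips IsOpen and re-enables interaction.
; It also exposes its interaction icon widget component through a getter.
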(event EventInteract
  (CallFunction|ToggleDoorEvent))

(event Custom|ToggleDoorEvent
  (bind _sm_door_01 (Variables|Default|GetSM_Door_01))
  (bind _relativerotation (Variables|/Script/Engine.SceneComponent|GetRelativeRotation _sm_door_01))
  ;[1 1 1] Use if CanOpen is true
  (if (Variables|Default|GetcanOpen)
    (Variables|Default|SetcanOpen false)
    ;[1 1 1] Open or Close? False is Open, True is Close
    (if (Variables|Default|GetisOpen)
      (bind _step (Timeline|TimelineRotation Reverse)
        (:Update
          (Transformation|SetRelativeRotation _sm_door_01 (Math|Rotator|MakeRotator (.roll _relativerotation) (.pitch _relativerotation) _step) false false))
        (:Finished
          ;[1 1 1] FinishOpening
          (Variables|Default|SetisOpen (not (Variables|Default|GetisOpen)))
          (Variables|Default|SetcanOpen true)))
      (else
        (Timeline|TimelineRotation Play)))))

(fn ConstructionScript)

(fn GetWidgetComponent
  (return (Variables|Default|GetInteractIconWidgetComponent)))