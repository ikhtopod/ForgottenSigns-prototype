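; Interactable prison cell door that swings open or closed when it receives an Interact event.
; A timeline lerps the door mesh's relative yaw between zero and MaxDoorRelativeRotationZ, playing forward to open and reversing to close.
; CanOpen blocks new toggles until the timeline finishes and flips IsOpen.
; Doors starting open snap to full rotation on BeginPlay, and a getter exposes the interact icon widget.
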(event EventBeginPlay
  (Init|InitDoor))

(event EventInteract
  (CallFunction|ToggleDoorEvent))

(event Custom|ToggleDoorEvent
  (bind _sm_celldoor_01 (Variables|Default|GetSM_CellDoor_01))
  (bind _relativerotation (Variables|/Script/Engine.SceneComponent|GetRelativeRotation _sm_celldoor_01))
  ;[1 1 1] Use if CanOpen is true
  (if (Variables|Default|GetcanOpen)
    (Variables|Default|SetcanOpen false)
    ;[1 1 1] Open or Close? False is Open, True is Close
    (Utilities|BranchFlip (Variables|Default|GetisOpen)
      (:false
        (bind _alpha (Timeline|TimelineRotation Play)
          (:Update
            (Transformation|SetRelativeRotation _sm_celldoor_01 (Math|Rotator|MakeRotator (.roll _relativerotation) (.pitch _relativerotation) (Math|Float|Lerp 0.0 (Variables|Default|GetmaxDoorRelativeRotationZ) _alpha)) false false))
          (:Finished
            ;[1 1 1] FinishOpening
            (Variables|Default|SetisOpen (not (Variables|Default|GetisOpen)))
            (Variables|Default|SetcanOpen true))))
      (:true
        (Timeline|TimelineRotation Reverse)))))

(fn ConstructionScript)

(fn InitDoor
  (if (Variables|Default|GetisOpen)
    (Reset|HardResetDoor)))

(fn HardResetDoor
  (bind _timelinerotation (Variables|Default|GetTimelineRotation))
  (bind _sm_celldoor_01 (Variables|Default|GetSM_CellDoor_01))
  (bind _relativerotation (Variables|/Script/Engine.SceneComponent|GetRelativeRotation _sm_celldoor_01))
  ;[1 1 1] Door Relative Rotation
  (Transformation|SetRelativeRotation _sm_celldoor_01 (Math|Rotator|MakeRotator (.roll _relativerotation) (.pitch _relativerotation) (Variables|Default|GetmaxDoorRelativeRotationZ)) false false)
  ;[1 1 1] Timeline to End
  (Components|Timeline|SetPlaybackPosition _timelinerotation (Components|Timeline|GetTimelineLength _timelinerotation) false true))

(fn GetWidgetComponent
  (return (Variables|Default|GetInteractIconWidgetComponent)))