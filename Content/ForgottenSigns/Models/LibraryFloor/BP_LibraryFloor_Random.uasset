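; BP_LibraryFloor_Random is a library floor Blueprint that shows a randomly chosen floor mesh from its LibraryFloors array.
; On BeginPlay it picks a random index into CurrentLibraryFloor, then assigns that mesh to LibraryFloorComponent.
; The construction script applies the current index without re-rolling, and the mesh is only set when the array is not empty.
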(event EventBeginPlay
  (CallFunction|InitCurrentLibraryFloor)
  (CallFunction|SetStaticMeshbyCurrentIndex))

(fn ConstructionScript
  (CallFunction|SetStaticMeshbyCurrentIndex))

(fn SetStaticMeshbyCurrentIndex
  (if (> (Utilities|Array|Length (Variables|Default|GetlibraryFloors)) 0)
    (Components|StaticMesh|SetStaticMesh (Variables|Default|GetlibraryFloorComponent) (Utilities|Array|Get(acopy) (Variables|Default|GetlibraryFloors) (Variables|Default|GetcurrentLibraryFloor)))))

(fn InitCurrentLibraryFloor
  (Variables|Default|SetcurrentLibraryFloor (Math|Random|RandomIntegerinRange 0 (Math|Integer|Max(Integer) 0 (Utilities|Array|LastIndex (Variables|Default|GetlibraryFloors))))))