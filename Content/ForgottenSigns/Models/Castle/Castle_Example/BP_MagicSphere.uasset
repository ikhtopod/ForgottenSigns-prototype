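; BP_MagicSphere is an animated castle example prop made of a magic sphere and three rings that spin continuously.
; Each Tick scales Speed by delta time and applies it as world rotation, keeping the spin frame-rate independent.
; The sphere rolls, RingY yaws, and RingX and RingZ both pitch, all at the same rate.
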(event EventTick
  (params (DeltaSeconds :type Float%20%28single-precision%29))
  (Variables|Default|SetspeedRot (* DeltaSeconds (Variables|Default|Getspeed)))
  (Transformation|AddWorldRotation (Variables|Default|GetCastle_Example_MagicSphere) (Math|Rotator|MakeRotator (Variables|Default|GetspeedRot) 0.0 0.0) false false)
  (Transformation|AddWorldRotation (Variables|Default|GetCastle_Example_RingX) (Math|Rotator|MakeRotator 0.0 (Variables|Default|GetspeedRot) 0.0) false false)
  (Transformation|AddWorldRotation (Variables|Default|GetCastle_Example_RingY) (Math|Rotator|MakeRotator 0.0 0.0 (Variables|Default|GetspeedRot)) false false)
  (Transformation|AddWorldRotation (Variables|Default|GetCastle_Example_RingZ) (Math|Rotator|MakeRotator 0.0 (Variables|Default|GetspeedRot) 0.0) false false))

(fn ConstructionScript)