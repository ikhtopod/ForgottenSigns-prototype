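; BP_Book_01 is an explorable book actor whose two covers can swing open and closed.
; ToggleBookEvent plays or reverses a timeline that lerps both cover meshes to mirrored pitch angles, with CanOpen blocking retriggers until it finishes.
; On BeginPlay it snaps an initially open book to the timeline's end and builds an explore message from its display name.
; It exposes that message and an icon widget through getters, while the Explore event itself is empty.
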(event EventBeginPlay
  (Init|InitBook)
  (CallFunction|InitExploreMessage))

(event EventExplore)

(event Custom|ToggleBookEvent
  (bind _sm_book_01_l (Variables|Default|GetSM_Book_01_L))
  (bind _sm_book_01_r (Variables|Default|GetSM_Book_01_R))
  (bind _relativerotation (Variables|/Script/Engine.SceneComponent|GetRelativeRotation _sm_book_01_l))
  (bind _relativerotation_2 (Variables|/Script/Engine.SceneComponent|GetRelativeRotation _sm_book_01_r))
  ;[1 1 1] Use if CanOpen is true
  (if (Variables|Toggle|GetcanOpen)
    (Variables|Toggle|SetcanOpen false)
    ;[1 1 1] Open or Close? False is Open, True is Close
    (Utilities|BranchFlip (Variables|Toggle|GetisOpen)
      (:false
        (bind _alpha (Timeline|TimelineRotation Play)
          (:Update
            ;[1 1 1] Cover R
            (Transformation|SetRelativeRotation _sm_book_01_r (Math|Rotator|MakeRotator (.roll _relativerotation_2) (Math|Float|Lerp 0.0 (Variables|Toggle|GetmaxBookCoverRelativeRotationZ) _alpha) (.yaw _relativerotation_2)) false false)
            ;[1 1 1] Cover L
            (Transformation|SetRelativeRotation _sm_book_01_l (Math|Rotator|MakeRotator (.roll _relativerotation) (* (Math|Float|Lerp 0.0 (Variables|Toggle|GetmaxBookCoverRelativeRotationZ) _alpha) -1.0) (.yaw _relativerotation)) false false))
          (:Finished
            ;[1 1 1] FinishOpening
            (Variables|Toggle|SetisOpen (not (Variables|Toggle|GetisOpen)))
            (Variables|Toggle|SetcanOpen true))))
      (:true
        (Timeline|TimelineRotation Reverse)))))

(fn ConstructionScript)

(fn InitBook
  (if (Variables|Toggle|GetisOpen)
    (Reset|HardResetBook)))

(fn HardResetBook
  (bind _maxbookcoverrelativerotationz (Variables|Toggle|GetmaxBookCoverRelativeRotationZ))
  (bind _sm_book_01_l (Variables|Default|GetSM_Book_01_L))
  (bind _sm_book_01_r (Variables|Default|GetSM_Book_01_R))
  (bind _timelinerotation (Variables|Default|GetTimelineRotation))
  (bind _relativerotation (Variables|/Script/Engine.SceneComponent|GetRelativeRotation _sm_book_01_l))
  (bind _relativerotation_2 (Variables|/Script/Engine.SceneComponent|GetRelativeRotation _sm_book_01_r))
  ;[1 1 1] Rotation Cover R
  (Transformation|SetRelativeRotation _sm_book_01_r (Math|Rotator|MakeRotator (.roll _relativerotation_2) _maxbookcoverrelativerotationz (.yaw _relativerotation_2)) false false)
  ;[1 1 1] Rotation Cover L
  (Transformation|SetRelativeRotation _sm_book_01_l (Math|Rotator|MakeRotator (.roll _relativerotation) (* _maxbookcoverrelativerotationz -1.0) (.yaw _relativerotation)) false false)
  ;[1 1 1] Timeline to End
  (Components|Timeline|SetPlaybackPosition _timelinerotation (Components|Timeline|GetTimelineLength _timelinerotation) false true))

(fn InitExploreMessage
  (Variables|Explore|SetexploreMessage (Utilities|Text|ToText(String) (Utilities|String|Append "Just the book with the title: " (Utilities|GetDisplayName self)))))

(fn GetExploreMessage
  (return (Variables|Explore|GetexploreMessage)))

(fn GetWidgetComponent
  (return (Variables|Default|GetExploreIconWidgetComponent)))