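; Inventory component that stores items as stackable slots up to a maximum slot count.
; Taking an item drains its quantity into matching stacks, then into new slots, leaving any excess on the item.
; A sort pass then merges slots by item class and re-splits them by max stack size.
; Dropping removes part or all of a slot and spawns that item class at the owner's location with the removed quantity.
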(fn TakeItems
  (params (item :type BP%20Inventory%20Item%20Object%20Reference%20%28by%20ref%29))
  (TakeItems|FillExistingSlots item)
  (TakeItems|FillFreeSlots item)
  (CallFunction|SortSlots))

(fn DropItem
  (params (slotIndex :type Integer) (countItems :type Integer))
  (Utilities|IsTrue (DropItem|IsValidInputDataforDropItem slotIndex countItems)
    (:true
      (bind (_classitem _quantity) (DropItem|ClearSlotData slotIndex countItems))
      (DropItem|SpawnDropbyClass _classitem _quantity))))

(fn HasEmptySlot
  (return (< (Utilities|Array|Length (Variables|Default|GetslotData)) (Variables|Default|GetmaxInventorySlots))))

(fn IsValidInputDataforDropItem
  (params (slotIndex :type Integer) (countItems :type Integer))
  (return (and (Utilities|Array|IsValidIndex (Variables|Default|GetslotData) slotIndex) (> countItems 0))))

(fn NeedDeleteEntireSlot
  (params (slotIndex :type Integer) (countItem :type Integer))
  (return (<= (.quantity (Utilities|Array|Get(acopy) (Variables|Default|GetslotData) slotIndex)) countItem)))

(fn ClearSlotData
  (params (slotIndex :type Integer) (countItems :type Integer))
  (if (DropItem|NeedDeleteEntireSlot slotIndex countItems)
    (bind (_classitem _quantity) (DropItem|ClearSlotData|DeleteEntireSlot slotIndex))
    (return _classitem _quantity)
    (else
      (bind (_classitem_2 _quantity_2) (DropItem|ClearSlotData|DeleteSomeItems slotIndex countItems))
      (return _classitem_2 _quantity_2))))

(fn SpawnDropbyClass
  (params (classItem :type BP%20Inventory%20Item%20Class%20Reference) (quantity :type Integer))
  (bind _returnvalue (Game|SpawnActorfromClass classItem (Math|Transform|MakeTransform (Transformation|GetActorLocation (Components|GetOwner)) "0, 0, 0" "1,1,1") "Undefined" 0 0))
  (Default|SetQuantity _returnvalue quantity)
  (return _returnvalue))

(fn DeleteEntireSlot
  (params (slotIndex :type Integer))
  (bind _slotdata (Variables|Default|GetslotData))
  (bind _output (Utilities|Array|Get(acopy) _slotdata slotIndex))
  (LocalVariables|SetspawnClass (.class (.itemdata _output)))
  (LocalVariables|SetquantityTmp (.quantity _output))
  (Utilities|Array|RemoveIndex (Variables|Default|GetslotData) slotIndex)
  (return (LocalVariables|GetspawnClass) (LocalVariables|GetquantityTmp)))

(fn DeleteSomeItems
  (params (slotIndex :type Integer) (countItems :type Integer))
  (bind _slotdata (Variables|Default|GetslotData))
  (bind _output (Utilities|Array|Get(acopy) _slotdata slotIndex))
  (LocalVariables|SetspawnClass (.class (.itemdata _output)))
  (|SetBy-RefVar (.quantity _output) (- (.quantity _output) countItems))
  (return (LocalVariables|GetspawnClass) countItems))

(fn FillExistingSlots
  (params (item :type BP%20Inventory%20Item%20Object%20Reference%20%28by%20ref%29))
  (bind _quantity (Default|GetQuantity item))
  (bind (_array_element _array_index) (Utilities|Array|ForEachLoopwithBreak (Variables|Default|GetslotData) :!label _label)
    (:LoopBody
      ;[1 1 1] Если элементов в дропе нет, то завершить перебор по инвентарю
      (Utilities|BranchFlip (Default|HasItems item)
        (:false
          (goto _label Break))
        (:true
          ;[1 1 1] Соответствует ли дроп элементу в заданном слоте
          (Utilities|IsTrue (CallFunction|EqualsSInventoryItemData (Variables|/Game/ForgottenSigns/Gameplay/Inventory/BP_InventoryItem.BP_InventoryItem_C|GetitemData item) (.itemdata _array_element))
            (:true
              ;[1 1 1] Забираем элементы из дропа
              (LocalVariables|SetminTmp (Math|Integer|Min(Integer) _quantity (- (.maxstacksize (.itemdata (Utilities|Array|Get(acopy) (Variables|Default|GetslotData) _array_index))) (.quantity (Utilities|Array|Get(acopy) (Variables|Default|GetslotData) _array_index)))))
              (Default|SetQuantity item (- _quantity (LocalVariables|GetminTmp)))
              ;[1 1 1] Добавляем элементы в слот
              (|SetBy-RefVar (.quantity (Utilities|Array|Get(acopy) (Variables|Default|GetslotData) _array_index)) (+ (LocalVariables|GetminTmp) (.quantity (Utilities|Array|Get(acopy) (Variables|Default|GetslotData) _array_index)))))))))))

(fn FillFreeSlots
  (params (item :type BP%20Inventory%20Item%20Object%20Reference%20%28by%20ref%29))
  (bind _quantity (Default|GetQuantity item))
  (while (and (Default|HasItems item) (CallFunction|HasEmptySlot))
    (LocalVariables|SetminTmp (Math|Integer|Min(Integer) _quantity (.maxstacksize (Variables|/Game/ForgottenSigns/Gameplay/Inventory/BP_InventoryItem.BP_InventoryItem_C|GetitemData item))))
    (Default|SetQuantity item (- _quantity (LocalVariables|GetminTmp)))
    (Utilities|Array|Add (Variables|Default|GetslotData) (Utilities|Struct|MakeS_InventorySlotData (Variables|/Game/ForgottenSigns/Gameplay/Inventory/BP_InventoryItem.BP_InventoryItem_C|GetitemData item) (LocalVariables|GetminTmp)))))

(fn SortSlots
  (bind _tmpslotdata (LocalVariables|GettmpSlotData))
  (bind _returnvalue (Utilities|Array|LastIndex _tmpslotdata))
  (bind _output (Utilities|Array|Get(acopy) _tmpslotdata _returnvalue))
  ;[1 1 1] Не сортировать, если в slotData меньше двух элементов
  (Utilities|IsTrue (> (Utilities|Array|Length (Variables|Default|GetslotData)) 1)
    (:true
      (while (> (Utilities|Array|Length (Variables|Default|GetslotData)) 0) ; Цикл работает до тех пор, пока slotData не опустеет
        ;[1 1 1] Добавить в tmpSlotData первый элемент из slotData, из которого он же будет удален. Данный элемент будет считаться "стартовым" для сравнения типов и подсчета общего количества элементов данного типа.
        (Utilities|Array|Add (LocalVariables|GettmpSlotData) (Utilities|Array|Get(acopy) (Variables|Default|GetslotData)))
        (Utilities|Array|RemoveIndex (Variables|Default|GetslotData))
        (for (_array_element _array_index) (Variables|Default|GetslotData)
          (LocalVariables|SettmpSlot _array_element)
          ;[1 1 1] Если какой-либо элемент slotData, соответствует (по классу) последнему добавленному в tmpSlotData элементу, то последнему в tmpSlotData надо повысить quantity, соответствующее quantity элемента в slotData.
          (Utilities|IsTrue (== (.class (.itemdata (LocalVariables|GettmpSlot))) (.class (.itemdata _output)))
            (:true
              (Utilities|Array|Add (LocalVariables|GetindicesForRemove) _array_index)
              (|SetBy-RefVar (.quantity _output) (+ (.quantity (LocalVariables|GettmpSlot)) (.quantity _output))))))
        ;[1 1 1] Удалить (по индексу) из slotData добавленные в tmpSlotData элементы
        (bind _arrayelement (Utilities|Array|ReverseforEachLoop (LocalVariables|GetindicesForRemove))
          (:LoopBody
            (Utilities|Array|RemoveIndex (Variables|Default|GetslotData) _arrayelement))
          (:Completed
            (Utilities|Array|Clear (LocalVariables|GetindicesForRemove)))))
      ;[1 1 1] Распределение собранных в tmpSlotData элементов по slotData
      (for _array_element_2 (LocalVariables|GettmpSlotData)
        (bind _output_get (LocalVariables|SettmpSlot _array_element_2))
        (while (> (.quantity _output_get) (.maxstacksize (.itemdata _output_get)))
          ;;[1 1 1] Заполнить слоты по максимальным количествам элементов
          (Utilities|Array|Add (Variables|Default|GetslotData) (Utilities|Struct|MakeS_InventorySlotData (Utilities|Struct|MakeS_InventoryItemData (.name (.itemdata (LocalVariables|GettmpSlot))) (.description (.itemdata (LocalVariables|GettmpSlot))) (.maxstacksize (.itemdata (LocalVariables|GettmpSlot))) (.thumbnail (.itemdata (LocalVariables|GettmpSlot))) (.class (.itemdata (LocalVariables|GettmpSlot)))) (.maxstacksize (.itemdata (LocalVariables|GettmpSlot)))))
          (|SetBy-RefVar (.quantity (LocalVariables|GettmpSlot)) (- (.quantity (LocalVariables|GettmpSlot)) (.maxstacksize (.itemdata (LocalVariables|GettmpSlot))))))
        ;;[1 1 1] Заполнить один слот остатками элементов
        (Utilities|IsTrue (> (.quantity (LocalVariables|GettmpSlot)) 0)
          (:true
            (Utilities|Array|Add (Variables|Default|GetslotData) (LocalVariables|GettmpSlot)))))
      (Utilities|Array|Clear (LocalVariables|GettmpSlotData)))))