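; BP_InventoryLibrary is a Blueprint function library that provides equality checks for inventory item and slot structs.
; The item check compares every listed field, from name and description to stack size, thumbnail and class.
; The slot check repeats that field-by-field comparison on the nested item data, without calling the item function, and also requires equal quantity.
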(fn EqualsSInventoryItemData
  (params (first :type S%20Inventory%20Item%20Data%20Structure) (second :type S%20Inventory%20Item%20Data%20Structure))
  (bind (_name _description _maxstacksize _thumbnail _class) (Utilities|Struct|BreakS_InventoryItemData second))
  (bind (_name_2 _description_2 _maxstacksize_2 _thumbnail_2 _class_2) (Utilities|Struct|BreakS_InventoryItemData first))
  (return (Math|Boolean|ANDBoolean (Utilities|Enum|Equal(Enum) _name_2 _name) (Utilities|Enum|Equal(Enum) _description_2 _description) (== _maxstacksize_2 _maxstacksize) (== _thumbnail_2 _thumbnail) (== _class_2 _class))))

(fn EqualsSInventorySlotData
  (params (first :type S%20Inventory%20Slot%20Data%20Structure) (second :type S%20Inventory%20Slot%20Data%20Structure))
  (bind (_itemdata _quantity) (Utilities|Struct|BreakS_InventorySlotData first))
  (bind (_itemdata_2 _quantity_2) (Utilities|Struct|BreakS_InventorySlotData second))
  (return (Math|Boolean|ANDBoolean (Utilities|Enum|Equal(Enum) (.name _itemdata) (.name _itemdata_2)) (Utilities|Enum|Equal(Enum) (.description _itemdata) (.description _itemdata_2)) (== (.maxstacksize _itemdata) (.maxstacksize _itemdata_2)) (== (.thumbnail _itemdata) (.thumbnail _itemdata_2)) (== (.class _itemdata) (.class _itemdata_2)) (== _quantity _quantity_2))))