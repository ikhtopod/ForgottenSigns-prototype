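; BP_StorageBase is a base storage container that the player interacts with to open a storage screen.
; On BeginPlay it caches the game instance, gives its inventory component a random slot limit and passes that component's name to its icon widget.
; Interacting while unpaused pauses the game, opens UI_Storage linking the player's and container's inventories, and switches to UI-only input with a visible cursor.
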(event EventBeginPlay
  (CallFunction|InitMainGameInstance)
  (bind _output_get (Variables|Default|SetmaxInventorySlots (Math|Random|RandomIntegerinRange 1 9)))
  (Variables|/Game/ForgottenSigns/Gameplay/Inventory/BP_InventoryComponent.BP_InventoryComponent_C|SetmaxInventorySlots (Variables|Default|GetBP_InventoryComponent) _output_get)
  (CallFunction|UpdateUIInformation))

(event EventInteract
  (CallFunction|ShowUI))

(fn ConstructionScript)

(fn UpdateUIInformation
  (Default|UpdateStorageIconInformation (Variables|Default|GetStorageIconWidgetComponent) (Variables|/Game/ForgottenSigns/Gameplay/Inventory/BP_InventoryComponent.BP_InventoryComponent_C|Getname (Variables|Default|GetBP_InventoryComponent))))

(fn InitMainGameInstance
  (bind _asmain_game_instance (Utilities|Casting|CastToMainGameInstance (Game|GetGameInstance)))
  (Variables|Default|SetmainGameInstance _asmain_game_instance))

(fn ShowUI
  (bind _returnvalue (Game|GetPlayerController 0))
  (Utilities|IsFalse (Game|IsGamePaused)
    (:false
      (Game|SetGamePaused true)
      (Variables|/Script/Engine.PlayerController|SetbShowMouseCursor _returnvalue true)
      (bind _asbp_default_player (Utilities|Casting|CastToBP_DefaultPlayer (Game|GetPlayerCharacter 0)))
      (bind _returnvalue_2 (UserInterface|CreateWidget "/Game/ForgottenSigns/Gameplay/Storage/UI_Storage.UI_Storage_C" _returnvalue (Variables|/Game/ForgottenSigns/Characters/Player/BP_DefaultPlayer.BP_DefaultPlayer_C|GetBP_InventoryComponent _asbp_default_player) (Variables|Default|GetBP_InventoryComponent)))
      (UserInterface|Viewport|AddtoViewport _returnvalue_2 0)
      (Input|SetInputModeUIOnly (Game|GetPlayerController 0) _returnvalue_2 "DoNotLock"))))

(fn GetWidgetComponent
  (return (Variables|Default|GetStorageIconWidgetComponent)))