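; Day-night cycle actor that animates sun, sky and fog while tracking the in-game day and time.
; A timeline starts at StartDayTime, runs at DayRate, and each update drives directional light rotation and intensity, sky light, height fog density and sky sphere sun direction.
; It also sets the CurrentTime timespan and day-interval enum; on finish it increments Day and replays.
; A looping timer periodically recaptures the sky light.
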(event Custom|RecaptureSkyLight
  ;[1 1 1] Recapture Sky
  (Class|SkyLightComponent|RecaptureSky (Variables|/Script/Engine.SkyLight|GetLightComponent (Variables|SkyLight|GetskyLight))))

(event EventBeginPlay
  (Utilities|FlowControl|Sequence
    (:then_0
      ;[1 1 1] DayLightCycle Timeline
      (bind (_direction _directionallightrotationpitch _directionallightrotationyaw _directionallightintensity _skylightintensity _exponentialheightfogdensity _time _dayinterval) (Timeline|DayNightCycle_Timeline SetNewTime)
        (:Update
          (CallFunction|UpdateCycle _directionallightrotationpitch _directionallightrotationyaw _directionallightintensity _skylightintensity _exponentialheightfogdensity _time _dayinterval))
        (:Finished
          (Time|UpdateDay) ; Update Day and Start Timeline from begin
          (Timeline|DayNightCycle_Timeline PlayFromStart))))
    (:then_1
      ;[1 1 1] Recapture Sky
      (Utilities|Time|SetTimerbyEvent (delegate Custom|RecaptureSkyLight) (Variables|SkyLight|GetrecaptureSkyLightTime) true))))

(fn ConstructionScript
  (Components|Timeline|SetPlayRate (Variables|Default|GetDayNightCycle_Timeline) (Variables|Time|Timeline|GetdayRate)))

(fn UpdateTimespan
  (params (second :type Float%20%28single-precision%29))
  (Variables|Time|SetcurrentTime (Math|Timespan|MakeTimespan (Variables|Time|Getday) 0 0 (Math|Float|Truncate second))))

(fn UpdateDay
  (Math|Integer|IncrementInt (Variables|Time|Getday)))

(fn UpdateDirectionalLight
  (params (newRotationPitch :type Float%20%28single-precision%29) (newRotationYaw :type Float%20%28single-precision%29) (newIntensity :type Float%20%28single-precision%29))
  (bind _directionallight (Variables|DirectionalLight|GetdirectionalLight))
  (Transformation|SetActorRotation _directionallight (Math|Rotator|MakeRotator 0.0 newRotationPitch newRotationYaw))
  (Rendering|Components|Light|SetIntensity (Variables|/Script/Engine.Light|GetLightComponent _directionallight) newIntensity))

(fn UpdateSkyLight
  (params (newIntensity :type Float%20%28single-precision%29))
  (Rendering|Components|Light|SetIntensity (Variables|/Script/Engine.SkyLight|GetLightComponent (Variables|SkyLight|GetskyLight)) newIntensity))

(fn UpdateExponentialHeightFog
  (params (density :type Float%20%28single-precision%29))
  (Class|ExponentialHeightFogComponent|SetFogDensity (Variables|/Script/Engine.ExponentialHeightFog|GetComponent (Variables|ExponentialHeightFog|GetexponentialHeightFog)) density))

(fn UpdateSkySphere
  (Default|UpdateSunDirection (Variables|SkySphere|GetskySphere)))

(fn UpdateCycle
  (params (newRotationPitch :type Float%20%28single-precision%29) (newRotationYaw :type Float%20%28single-precision%29) (newIntensityDirectionalLight :type Float%20%28single-precision%29) (newIntensitySkyLight :type Float%20%28single-precision%29) (densityExponentialHeightFog :type Float%20%28single-precision%29) (time :type Float%20%28single-precision%29) (dayInterval :type Float%20%28single-precision%29))
  (DirectionalLight|UpdateDirectionalLight newRotationPitch newRotationYaw newIntensityDirectionalLight)
  (SkyLight|UpdateSkyLight newIntensitySkyLight)
  (ExponentialHeightFog|UpdateExponentialHeightFog densityExponentialHeightFog)
  (Time|UpdateTimespan time)
  (Time|UpdateDayInterval dayInterval)
  (SkySphere|UpdateSkySphere))

(fn UpdateDayInterval
  (params (newDayInterval :type Float%20%28single-precision%29))
  (Variables|Time|SetdayInterval (Utilities|Enum|ByteToEnumE_DayInterval (Math|Conversions|ToByte(Integer) (Math|Float|Truncate newDayInterval)))))