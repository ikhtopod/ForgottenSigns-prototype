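; First-person player character that handles movement, look, jump, crouch, run, object interaction and a pausing escape menu through control events.
; A camera line trace on use calls Interact on Interactable actors, or shows an animated message and calls Explore on Exploreable ones.
; A looping timer repeats the trace, toggling the hit actor's prompt widget against the crosshair.
; It creates its HUD, explore and escape-menu widgets on BeginPlay.
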(event Custom|ShowIconEvent
  ;[1 1 1] Init Using Message
  (ShowIcon|ShowIcon))

(event EventPossessed
  (params (NewController :type Controller%20Object%20Reference))
  ;[1 1 1] Possessed
  (CallFunction|CastControllertoPlayerController NewController))

(event EventUnpossessed
  (params (OldController :type Controller%20Object%20Reference))
  ;[1 1 1] Possessed
  (Variables|Default|SetcurrentPlayerController 0))

(event EventBeginPlay
  (Utilities|FlowControl|Sequence
    (:then_0
      ;[1 1 1] Possessed
      (CallFunction|CastControllertoPlayerController (Pawn|GetController)))
    (:then_1
      ;[1 1 1] Init UI
      (Init|InitPrevWidgetComponent)
      (Init|InitUIPlayerDefault)
      (Init|InitUIPlayerExplore)
      (Init|InitUIPlayerESCMenu))
    (:then_2
      ;[1 1 1] Init Using Message
      (bind _returnvalue (Utilities|Time|SetTimerbyEvent (delegate Custom|ShowIconEvent) (/ 1.0 (Variables|Icon|GetnumberOfTimesShowIcon)) true))
      (Variables|Icon|SetshowIconHandle _returnvalue))))

(event EventMoveForwardControl
  (params (AxisValue :type Float%20%28single-precision%29))
  ;[0 0 0] PlayerController
  ;;[1 1 1] Movement
  (Pawn|Input|AddMovementInput (Transformation|GetActorForwardVector) AxisValue false))

(event EventStopRunningControl
  ;[0 0 0] PlayerController
  ;;[1 1 1] Running
  (Variables|/Script/Engine.CharacterMovementComponent|SetMaxWalkSpeed (Variables|Character|GetCharacterMovement) (Variables|Walk|GetmaxWalkSpeedTmp)))

(event EventUseControl
  ;[0 0 0] PlayerController
  ;;[1 1 1] Using
  (bind (_washit _resulthit) (Using|LineTraceObject))
  (if _washit
    (Variables|Using|SetcurrentHitActor (.HitActor (Collision|BreakHitResult _resulthit)))
    (Utilities|FlowControl|Sequence
      (:then_0
        (bind _asinteractable (Utilities|Casting|CastToInteractable (Variables|Using|GetcurrentHitActor))
          (:then
            (Default|Interact _asinteractable))
          (:CastFailed
            (bind _asexploreable (Utilities|Casting|CastToExploreable (Variables|Using|GetcurrentHitActor)))
            (Using|ExploreReaction _asexploreable))))
      (:then_1
        (Variables|Using|SetcurrentHitActor 0) ; Reset currentHitActor
      ))))

(event EventToggleEscapeMenuControl
  ;[1 1 1] EscapeMenu with Pausing game
  (if (Utilities|Enum|Equal(Enum) (Widget|GetVisibility (Variables|UI|GetUI_PlayerESCMenu)) "Hidden")
    (EscapeMenu|ShowEscapeMenu)
    (else
      (EscapeMenu|HideEscapeMenu))))

(event EventMoveRightControl
  (params (AxisValue :type Float%20%28single-precision%29))
  ;[0 0 0] PlayerController
  ;;[1 1 1] Movement
  (Pawn|Input|AddMovementInput (Transformation|GetActorRightVector) AxisValue false))

(event EventTurnControl
  (params (AxisValue :type Float%20%28single-precision%29))
  ;[0 0 0] PlayerController
  ;;[1 1 1] Looking
  (Pawn|Input|AddControllerYawInput (* AxisValue (Variables|Mouse|GetmouseSensitivity) (Utilities|Time|GetWorldDeltaSeconds))))

(event EventLookUpControl
  (params (AxisValue :type Float%20%28single-precision%29))
  ;[0 0 0] PlayerController
  ;;[1 1 1] Looking
  (Pawn|Input|AddControllerPitchInput (* AxisValue (Variables|Mouse|GetmouseSensitivity) (Utilities|Time|GetWorldDeltaSeconds))))

(event EventJumpControl
  ;[0 0 0] PlayerController
  ;;[1 1 1] Jumping
  (Character|Jump))

(event EventStopJumpingControl
  ;[0 0 0] PlayerController
  ;;[1 1 1] Jumping
  (Character|StopJumping))

(event EventCrouchControl
  ;[0 0 0] PlayerController
  ;;[1 1 1] Crouch
  (Character|Crouch))

(event EventUnCrouchControl
  ;[0 0 0] PlayerController
  ;;[1 1 1] Crouch
  (Character|UnCrouch))

(event EventRunControl
  (bind _charactermovement (Variables|Character|GetCharacterMovement))
  ;[0 0 0] PlayerController
  ;;[1 1 1] Running
  (bind _output_get (Variables|Walk|SetmaxWalkSpeedTmp (Variables|/Script/Engine.CharacterMovementComponent|GetMaxWalkSpeed _charactermovement)))
  (Variables|/Script/Engine.CharacterMovementComponent|SetMaxWalkSpeed _charactermovement (* _output_get 1.5)))

(fn ConstructionScript)

(fn LineTraceObject
  (bind _camera (Variables|Components|GetCamera))
  (bind _returnvalue (Transformation|GetWorldLocation _camera))
  (bind (_outhit _returnvalue_2) (Collision|LineTraceForObjects _returnvalue (+ _returnvalue (* (Math|Vector|GetForwardVector (Transformation|GetWorldRotation _camera)) (Variables|Interact|GetinteractLength))) (Utilities|Array|MakeArray "ObjectTypeQuery1" "ObjectTypeQuery2") false 0 "None"))
  (return _returnvalue_2 _outhit))

(fn ShowIcon
  (bind (_washit _resulthit) (Using|LineTraceObject))
  ;[1 1 1] Show or Hide UIMessage
  (if _washit
    (bind _asihas_widget_component (Utilities|Casting|CastToIHasWidgetComponent (.HitActor (Collision|BreakHitResult _resulthit)))
      (:then
        (bind _widgetcomponent (Default|GetWidgetComponent _asihas_widget_component))
        (ShowIcon|ShowCurrentWidgetComponent _widgetcomponent)
        (Default|HideCrosshair (Variables|UI|GetUI_PlayerDefault)))
      (:CastFailed
        (ShowIcon|HidePrevWidgetComponent :!label _label)
        (Default|ShowCrosshair (Variables|UI|GetUI_PlayerDefault))))
    (else
      (goto _label))))

(fn InitPrevWidgetComponent
  (bind _pervwidgetcomponent (Variables|Icon|GetpervWidgetComponent))
  (if (Utilities|IsValid _pervwidgetcomponent)
    (Rendering|SetVisibility _pervwidgetcomponent false true)))

(fn InitUIPlayerDefault
  (bind _returnvalue (UserInterface|CreateWidget "/Game/ForgottenSigns/UI/Player/UI_PlayerDefault.UI_PlayerDefault_C"))
  (bind _output_get (Variables|UI|SetUI_PlayerDefault _returnvalue))
  (UserInterface|Viewport|AddtoViewport _output_get 0))

(fn HidePrevWidgetComponent
  (bind _pervwidgetcomponent (Variables|Icon|GetpervWidgetComponent))
  (Utilities|IsValid _pervwidgetcomponent
    (:Is%20Valid
      (if (Rendering|IsVisible _pervwidgetcomponent)
        (Rendering|SetVisibility (Variables|Icon|GetpervWidgetComponent) false true)))))

(fn ShowCurrentWidgetComponent
  (params (widgetComponent :type Widget%20Component%20Object%20Reference))
  (if (== (Variables|Icon|GetpervWidgetComponent) widgetComponent)
    _
    (else
      (ShowIcon|HidePrevWidgetComponent)
      (Variables|Icon|SetpervWidgetComponent widgetComponent)))
  (Utilities|IsValid (Variables|Icon|GetpervWidgetComponent)
    (:Is%20Valid
      (if (not (Rendering|IsVisible (Variables|Icon|GetpervWidgetComponent)))
        (Rendering|SetVisibility (Variables|Icon|GetpervWidgetComponent) true false)))))

(fn InitUIPlayerExplore
  (bind _returnvalue (UserInterface|CreateWidget "/Game/ForgottenSigns/UI/Player/UI_PlayerExplore.UI_PlayerExplore_C"))
  (bind _output_get (Variables|UI|SetUI_PlayerExplore _returnvalue))
  (UserInterface|Viewport|AddtoViewport _output_get 0))

(fn ExploreReaction
  (params (explorable :type Exploreable%20Interface))
  (bind _ui_playerexplore (Variables|UI|GetUI_PlayerExplore))
  (bind _ui_playerexplore_2 (Variables|UI|GetUI_PlayerExplore))
  (bind _ui_playerexplore_3 (Variables|UI|GetUI_PlayerExplore))
  (LocalVariables|SetexplorableObject explorable)
  ;[1 1 1] Update Message Text In UI
  (bind _message (Default|GetExploreMessage (LocalVariables|GetexplorableObject)))
  (Rendering|Components|TextRender|SetText (Variables|/Game/ForgottenSigns/UI/Player/UI_PlayerExplore.UI_PlayerExplore_C|GetexploreMessageText (Variables|UI|GetUI_PlayerExplore)) _message)
  (Utilities|FlowControl|Sequence
    (:then_0
      ;[1 1 1] StopAnimation
      (Utilities|IsTrue (Class|UserWidget|IsAnimationPlaying _ui_playerexplore (Variables|/Game/ForgottenSigns/UI/Player/UI_PlayerExplore.UI_PlayerExplore_C|GetHideExploreMessageTextAnimation _ui_playerexplore))
        (:true
          (Class|UserWidget|StopAnimation _ui_playerexplore_2 (Variables|/Game/ForgottenSigns/UI/Player/UI_PlayerExplore.UI_PlayerExplore_C|GetHideExploreMessageTextAnimation _ui_playerexplore_2)))))
    (:then_1
      ;[1 1 1] Play Animation
      (UserInterface|Animation|PlayAnimation _ui_playerexplore_3 (Variables|/Game/ForgottenSigns/UI/Player/UI_PlayerExplore.UI_PlayerExplore_C|GetHideExploreMessageTextAnimation _ui_playerexplore_3) 0.0 1 "Forward" 1.0 false))
    (:then_2
      ;[1 1 1] Run Explore Function
      (Default|Explore (LocalVariables|GetexplorableObject)))))

(fn InitUIPlayerESCMenu
  (bind _returnvalue (UserInterface|CreateWidget "/Game/ForgottenSigns/UI/Player/UI_PlayerESCMenu.UI_PlayerESCMenu_C"))
  (bind _output_get (Variables|UI|SetUI_PlayerESCMenu _returnvalue))
  (UserInterface|Viewport|AddtoViewport _output_get 0)
  (Widget|SetVisibility (Variables|UI|GetUI_PlayerESCMenu) "Hidden")
  (Widget|SetIsEnabled (Variables|UI|GetUI_PlayerESCMenu) false))

(fn ShowEscapeMenu
  (bind _currentplayercontroller (Variables|Default|GetcurrentPlayerController))
  (bind _ui_playerescmenu (Variables|UI|GetUI_PlayerESCMenu))
  (bind _ui_playerescmenu_2 (Variables|UI|GetUI_PlayerESCMenu))
  (Utilities|FlowControl|Sequence
    (:then_0
      ;[1 1 1] StopAnimation
      (Utilities|IsTrue (Class|UserWidget|IsPlayingAnimation _ui_playerescmenu_2)
        (:true
          (Class|UserWidget|StopAllAnimations _ui_playerescmenu_2))))
    (:then_1
      ;[1 1 1] Play Animation
      (UserInterface|Animation|PlayAnimation _ui_playerescmenu (Variables|/Game/ForgottenSigns/UI/Player/UI_PlayerESCMenu.UI_PlayerESCMenu_C|GetShowScreen _ui_playerescmenu) 0.0 1 "Forward" 1.0 false))
    (:then_2
      ;[1 1 1] Game Pause And Set Input Mode
      (Game|SetGamePaused true)
      (Input|SetInputModeUIOnly _currentplayercontroller (Variables|UI|GetUI_PlayerESCMenu) "DoNotLock")
      (Variables|/Script/Engine.PlayerController|SetbShowMouseCursor _currentplayercontroller true))))

(fn HideEscapeMenu
  (bind _currentplayercontroller (Variables|Default|GetcurrentPlayerController))
  (bind _ui_playerescmenu (Variables|UI|GetUI_PlayerESCMenu))
  (bind _ui_playerescmenu_2 (Variables|UI|GetUI_PlayerESCMenu))
  (Utilities|FlowControl|Sequence
    (:then_0
      ;[1 1 1] Set Input Mode
      (Variables|/Script/Engine.PlayerController|SetbShowMouseCursor _currentplayercontroller false)
      (Input|SetInputModeGameOnly _currentplayercontroller))
    (:then_1
      ;[1 1 1] StopAnimation
      (Utilities|IsTrue (Class|UserWidget|IsPlayingAnimation _ui_playerescmenu_2)
        (:true
          (Class|UserWidget|StopAllAnimations _ui_playerescmenu_2))))
    (:then_2
      ;[1 1 1] Play Animation
      (UserInterface|Animation|PlayAnimation _ui_playerescmenu (Variables|/Game/ForgottenSigns/UI/Player/UI_PlayerESCMenu.UI_PlayerESCMenu_C|GetHideScreen _ui_playerescmenu) 0.0 1 "Forward" 1.0 false))
    (:then_3
      ;[1 1 1] Game Unpause
      (Game|SetGamePaused false))))

(fn CastControllertoPlayerController
  (params (Object :type Object%20Object%20Reference))
  (bind _asplayer_controller (Utilities|Casting|CastToPlayerController Object))
  (Variables|Default|SetcurrentPlayerController _asplayer_controller))